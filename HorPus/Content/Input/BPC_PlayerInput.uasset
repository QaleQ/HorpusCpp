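; Player input component that turns Enhanced Input actions into movement, mouse look, pause, sneak, breath holding, interaction and night vision.
; It caches the player, controller, game mode and inventory component on BeginPlay, then forwards actions to them.
; Slot keys set the selected item, which Use equips, spends unlocking a traced door, or drops; interaction messages traced interactables.
; Night vision flip-flops camera HUD and post-process; it and unlocking also advance missions in the Tinker level.
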(event Custom|OnStartMakeSelectedSlotHighlighted
  ;[1 1 1] Inventory slots
  (bind _uiref (Variables|/Game/Blueprint/BP_GameMode.BP_GameMode_C|GetUIRef (Variables|Refs|GetGameModeRef))
    (:then
      (Default|SelectedSlot _uiref (stale Input|EnhancedActionEvents|EnhancedInputActionIA_Inventory_Slot4 _output_get))
      (Default|DisplayItemName (Variables|Default|GetBPC%20Inventory)))
    (:else)))

(event Input|EnhancedActionEvents|EnhancedInputActionIA_HoldBreath
  (params (ActionValue :type Boolean) (ElapsedSeconds :type Float%20%28double-precision%29) (TriggeredSeconds :type Float%20%28double-precision%29) (InputAction :type Input%20Action%20Object%20Reference :default "/Game/Input/Action/IA_HoldBreath.IA_HoldBreath"))
  ;[1 0 0.6611] Hold Breath
  (:Started
    (Audio|Components|Audio|Stop (Variables|/Game/Blueprint/BP_Player.BP_Player_C|GetEmitBreathSound (Variables|Refs|GetPlayerRef)))
    (Audio|Components|Audio|Stop (Variables|/Game/Blueprint/BP_Player.BP_Player_C|GetRegularBreathing (Variables|Refs|GetPlayerRef)))
    (Audio|PlaySound2D "/Game/Blueprint/Sounds/Breathing/Inhale.Inhale" 1.0 1.0 0.0 0 0 false))
  (:Canceled
    (Audio|PlaySound2D "/Game/Blueprint/Sounds/Breathing/Exhale.Exhale" 1.0 1.0 0.0 0 0 false :!label _label)
    (Components|Timeline|PlayfromStart (Variables|/Game/Blueprint/BP_Player.BP_Player_C|GetEmitBreathSound (Variables|Refs|GetPlayerRef)))
    (Audio|Components|Audio|Play (Variables|/Game/Blueprint/BP_Player.BP_Player_C|GetRegularBreathing (Variables|Refs|GetPlayerRef)) 0.0))
  (:Completed
    (goto _label)))

(event Input|EnhancedActionEvents|EnhancedInputActionIA_Look
  (params (ActionValue :type Vector%202D%20Structure) (ElapsedSeconds :type Float%20%28double-precision%29) (TriggeredSeconds :type Float%20%28double-precision%29) (InputAction :type Input%20Action%20Object%20Reference :default "/Game/Input/Action/IA_Look.IA_Look"))
  (bind _playercharacterref (Variables|Refs|GetPlayerCharacterRef))
  (bind _mousesens (Variables|DefaultValues|GetMouseSens))
  ;[1 1 1] Mouse look
  (:Triggered
    (Pawn|Input|AddControllerYawInput _playercharacterref (* (.x ActionValue) _mousesens))
    (Pawn|Input|AddControllerPitchInput _playercharacterref (* (.y ActionValue) _mousesens))))

(event Input|EnhancedActionEvents|EnhancedInputActionIA_UseItem
  (params (ActionValue :type Boolean) (ElapsedSeconds :type Float%20%28double-precision%29) (TriggeredSeconds :type Float%20%28double-precision%29) (InputAction :type Input%20Action%20Object%20Reference :default "/Game/Input/Action/IA_UseItem.IA_UseItem"))
  (bind _bpc_inventory (Variables|Default|GetBPC%20Inventory))
  (bind _bpc_inventory_2 (Variables|Default|GetBPC%20Inventory))
  (bind _playerref (Variables|Refs|GetPlayerRef))
  (bind _playerref_2 (Variables|Refs|GetPlayerRef))
  (bind _inventory (Variables|/Game/Inventory/BPC_inventory.BPC_inventory_C|Getinventory _bpc_inventory))
  (bind _slotselected (Variables|/Game/Blueprint/BP_Player.BP_Player_C|GetSlotSelected _playerref))
  (bind _slotselected_2 (Variables|/Game/Blueprint/BP_Player.BP_Player_C|GetSlotSelected _playerref_2))
  (bind _output (Utilities|Array|Get(acopy) _inventory _slotselected))
  ;[1 1 1] Use Item (aka spawn the Active Item for the Collectable one) if its equipable it calls equip item instead
  (:Started
    (if (Variables|/Game/Blueprint/BP_GameMode.BP_GameMode_C|GetHasBackpack (Variables|Refs|GetGameModeRef))
      (if (Utilities|IsValidClass (.itemclass _output))
        (if (.equipable _output)
          (Default|EquipItem _bpc_inventory_2 (.sneaklevel _output) _slotselected_2)
          (Audio|PlaySoundatLocation "/Game/Inventory/Sounds/Equip.Equip" (Transformation|GetActorLocation _playerref_2) "0, 0, 0" 1.0 1.0 0.0 0 0 0 0)
          (elif (.usable _output)
            (bind _hitactor (Default|LineTrace (Variables|Refs|GetPlayerRef)))
            (bind _asbp_door_snap (Utilities|Casting|CastToBP_Door_Snap _hitactor))
            (Variables|/Game/Interactable/BP_Door_Snap.BP_Door_Snap_C|SetIsUnlocked _asbp_door_snap true)
            (Default|RemoveItemfromInventory _bpc_inventory_2 _slotselected_2)
            (Audio|PlaySoundatLocation "/Game/Interactable/SFX/Unlock.Unlock" (Transformation|GetActorLocation _asbp_door_snap) "0, 0, 0" 1.0 1.0 0.3 0 0 0 0)
            (bind _returnvalue (Game|GetCurrentLevelName true))
            (if (Utilities|Enum|Equal(Enum) _returnvalue "Tinker")
              (Utilities|FlowControl|DoOnce false
                (:Completed
                  (bind _asbp_player (Utilities|Casting|CastToBP_Player (Game|Player|GetPlayerPawn 0)))
                  (Default|GetNextMission (Variables|Refs|GetGameModeRef) (Variables|/Game/Blueprint/BP_Player.BP_Player_C|GetAlwaysVisibleUIRef _asbp_player)))))
            (else
              (Default|DropItem _bpc_inventory_2 (.activeactorspawn _output))
              (Default|RemoveItemfromInventory (Variables|Default|GetBPC%20Inventory) (Variables|/Game/Blueprint/BP_Player.BP_Player_C|GetSlotSelected (Variables|Refs|GetPlayerRef)))
              (Audio|PlaySoundatLocation "/Game/Inventory/Sounds/DropItem.DropItem" (Transformation|GetActorLocation _playerref_2) "0, 0, 0" 1.0 1.0 0.0 0 0 0 0))))))))

(event Input|EnhancedActionEvents|EnhancedInputActionIA_Move
  (params (ActionValue :type Vector%202D%20Structure) (ElapsedSeconds :type Float%20%28double-precision%29) (TriggeredSeconds :type Float%20%28double-precision%29) (InputAction :type Input%20Action%20Object%20Reference :default "/Game/Input/Action/IA_Move.IA_Move"))
  (bind _playerref (Variables|Refs|GetPlayerRef))
  ;[1 1 1] Add Mapping Context to steer the player
  (:Triggered
    (if (not (Class|Pawn|IsMoveInputIgnored (Variables|Refs|GetPlayerRef)))
      (Default|PlayFootstepTimeline (Variables|Refs|GetPlayerRef) true)
      (Utilities|FlowControl|Sequence
        (:then_0
          (Pawn|Input|AddMovementInput _playerref (Transformation|GetActorForwardVector _playerref) (.x ActionValue) false))
        (:then_1
          (Pawn|Input|AddMovementInput _playerref (Transformation|GetActorRightVector _playerref) (.y ActionValue) false)))))
  (:Canceled
    (Default|PlayFootstepTimeline (Variables|Refs|GetPlayerRef) false :!label _label))
  (:Completed
    (goto _label)))

(event Input|EnhancedActionEvents|EnhancedInputActionIA_Nightvision
  (params (ActionValue :type Boolean) (ElapsedSeconds :type Float%20%28double-precision%29) (TriggeredSeconds :type Float%20%28double-precision%29) (InputAction :type Input%20Action%20Object%20Reference :default "/Game/Input/Action/IA_Nightvision.IA_Nightvision"))
  (bind _playerref (Variables|Refs|GetPlayerRef))
  (bind _gamemoderef (Variables|Refs|GetGameModeRef))
  (bind _postprocess (Variables|/Game/Blueprint/BP_Player.BP_Player_C|GetPostProcess _playerref))
  ;[1 1 1] Toggle Night Vision
  (:Started
    (if (Variables|/Game/Blueprint/BP_GameMode.BP_GameMode_C|GetHasCamera _gamemoderef)
      _
      (else
        _))
    (Utilities|FlowControl|Sequence
      (:then_0
        (bind _returnvalue (Game|GetCurrentLevelName true))
        (if (Utilities|Enum|Equal(Enum) _returnvalue "Tinker")
          (Utilities|FlowControl|DoOnce false
            (:Completed
              (bind _asbp_player (Utilities|Casting|CastToBP_Player (Game|Player|GetPlayerPawn 0)))
              (Default|GetNextMission (Variables|Refs|GetGameModeRef) (Variables|/Game/Blueprint/BP_Player.BP_Player_C|GetAlwaysVisibleUIRef _asbp_player))))))
      (:then_1
        (Utilities|FlowControl|FlipFlop
          (:A
            (bind _returnvalue_2 (UserInterface|CreateWidget "/Game/UI/NightVision/BPW_CameraHUD.BPW_CameraHUD_C" (Variables|Refs|GetPlayerControllerRef)))
            (Variables|/Game/Blueprint/BP_GameMode.BP_GameMode_C|SetCameraHUD _gamemoderef _returnvalue_2)
            (UserInterface|Viewport|AddtoViewport _returnvalue_2 0)
            (Widget|SetVisibility _returnvalue_2 "Visible")
            (Variables|/Script/Engine.PostProcessComponent|SetbEnabled _postprocess true))
          (:B
            (Widget|SetVisibility _returnvalue_2 "Hidden")
            (Variables|/Script/Engine.PostProcessComponent|SetbEnabled _postprocess false)))))))

(event Input|EnhancedActionEvents|EnhancedInputActionIA_Inventory_Slot1
  (params (ActionValue :type Boolean) (ElapsedSeconds :type Float%20%28double-precision%29) (TriggeredSeconds :type Float%20%28double-precision%29) (InputAction :type Input%20Action%20Object%20Reference :default "/Game/Input/Action/IA_Inventory_Slot1.IA_Inventory_Slot1"))
  ;[1 1 1] Inventory slots
  (:Started
    (Variables|/Game/Blueprint/BP_Player.BP_Player_C|SetSlotSelected (Variables|Refs|GetPlayerRef) 0)
    (bind _uiref (Variables|/Game/Blueprint/BP_GameMode.BP_GameMode_C|GetUIRef (Variables|Refs|GetGameModeRef))
      (:then
        (Default|SelectedSlot _uiref (stale Input|EnhancedActionEvents|EnhancedInputActionIA_Inventory_Slot4 _output_get))
        (Default|DisplayItemName (Variables|Default|GetBPC%20Inventory)))
      (:else))))

(event Input|EnhancedActionEvents|EnhancedInputActionIA_Inventory_Slot2
  (params (ActionValue :type Boolean) (ElapsedSeconds :type Float%20%28double-precision%29) (TriggeredSeconds :type Float%20%28double-precision%29) (InputAction :type Input%20Action%20Object%20Reference :default "/Game/Input/Action/IA_Inventory_Slot2.IA_Inventory_Slot2"))
  ;[1 1 1] Inventory slots
  (:Started
    (Variables|/Game/Blueprint/BP_Player.BP_Player_C|SetSlotSelected (Variables|Refs|GetPlayerRef) 1)
    (bind _uiref (Variables|/Game/Blueprint/BP_GameMode.BP_GameMode_C|GetUIRef (Variables|Refs|GetGameModeRef))
      (:then
        (Default|SelectedSlot _uiref (stale Input|EnhancedActionEvents|EnhancedInputActionIA_Inventory_Slot4 _output_get))
        (Default|DisplayItemName (Variables|Default|GetBPC%20Inventory)))
      (:else))))

(event Input|EnhancedActionEvents|EnhancedInputActionIA_Inventory_Slot3
  (params (ActionValue :type Boolean) (ElapsedSeconds :type Float%20%28double-precision%29) (TriggeredSeconds :type Float%20%28double-precision%29) (InputAction :type Input%20Action%20Object%20Reference :default "/Game/Input/Action/IA_Inventory_Slot3.IA_Inventory_Slot3"))
  ;[1 1 1] Inventory slots
  (:Started
    (Variables|/Game/Blueprint/BP_Player.BP_Player_C|SetSlotSelected (Variables|Refs|GetPlayerRef) 2)
    (bind _uiref (Variables|/Game/Blueprint/BP_GameMode.BP_GameMode_C|GetUIRef (Variables|Refs|GetGameModeRef))
      (:then
        (Default|SelectedSlot _uiref (stale Input|EnhancedActionEvents|EnhancedInputActionIA_Inventory_Slot4 _output_get))
        (Default|DisplayItemName (Variables|Default|GetBPC%20Inventory)))
      (:else))))

(event Input|EnhancedActionEvents|EnhancedInputActionIA_Inventory_Slot4
  (params (ActionValue :type Boolean) (ElapsedSeconds :type Float%20%28double-precision%29) (TriggeredSeconds :type Float%20%28double-precision%29) (InputAction :type Input%20Action%20Object%20Reference :default "/Game/Input/Action/IA_Inventory_Slot4.IA_Inventory_Slot4"))
  ;[1 1 1] Inventory slots
  (:Started
    (bind _output_get (Variables|/Game/Blueprint/BP_Player.BP_Player_C|SetSlotSelected (Variables|Refs|GetPlayerRef) 3))
    (bind _uiref (Variables|/Game/Blueprint/BP_GameMode.BP_GameMode_C|GetUIRef (Variables|Refs|GetGameModeRef))
      (:then
        (Default|SelectedSlot _uiref _output_get)
        (Default|DisplayItemName (Variables|Default|GetBPC%20Inventory)))
      (:else))))

(event Input|EnhancedActionEvents|EnhancedInputActionIA_PauseGame
  (params (ActionValue :type Boolean) (ElapsedSeconds :type Float%20%28double-precision%29) (TriggeredSeconds :type Float%20%28double-precision%29) (InputAction :type Input%20Action%20Object%20Reference :default "/Game/Input/Action/IA_PauseGame.IA_PauseGame"))
  (bind _playercontrollerref (Variables|Refs|GetPlayerControllerRef))
  ;[1 1 1] Pause game
  (:Started
    (Utilities|IsValid (Variables|WidgetRefs|GetPauseMenuRef)
      (:Is%20Valid
        _)
      (:Is%20Not%20Valid
        (bind _returnvalue (UserInterface|CreateWidget "/Game/UI/BPW_PauseMenu.BPW_PauseMenu_C"))
        (Variables|WidgetRefs|SetPauseMenuRef _returnvalue)))
    (Variables|/Script/Engine.PlayerController|SetbShowMouseCursor _playercontrollerref true)
    (Input|SetInputModeUIOnly _playercontrollerref (Variables|WidgetRefs|GetPauseMenuRef) "DoNotLock" false)
    (UserInterface|Viewport|AddtoViewport (Variables|WidgetRefs|GetPauseMenuRef) 0)
    (Game|SetGamePaused true)))

(event Input|EnhancedActionEvents|EnhancedInputActionIA_Sneak
  (params (ActionValue :type Boolean) (ElapsedSeconds :type Float%20%28double-precision%29) (TriggeredSeconds :type Float%20%28double-precision%29) (InputAction :type Input%20Action%20Object%20Reference :default "/Game/Input/Action/IA_Sneak.IA_Sneak"))
  ;[1 1 1] Sneak
  (:Started
    (Default|Sneaking (Variables|Refs|GetPlayerRef) ActionValue)))

(event Input|EnhancedActionEvents|EnhancedInputActionIA_Interact
  (params (ActionValue :type Boolean) (ElapsedSeconds :type Float%20%28double-precision%29) (TriggeredSeconds :type Float%20%28double-precision%29) (InputAction :type Input%20Action%20Object%20Reference :default "/Game/Input/Action/IA_Interact.IA_Interact"))
  ;[1 1 1] Cast trace from the camera when input
  (:Started
    (bind _hitactor (Default|LineTrace (Variables|Refs|GetPlayerRef)))
    (if (Utilities|DoesObjectImplementInterface _hitactor "/Game/Interactable/BPI_Interactable.BPI_Interactable_C")
      ;[0 0 0] Check if actor is interactable
      (Class|BPIInteractable|Interact(Message) _hitactor))))

(event Input|EnhancedActionEvents|EnhancedInputActionIA_DropItem
  (params (ActionValue :type Boolean) (ElapsedSeconds :type Float%20%28double-precision%29) (TriggeredSeconds :type Float%20%28double-precision%29) (InputAction :type Input%20Action%20Object%20Reference :default "/Game/Input/Action/IA_DropItem.IA_DropItem"))
  (bind _bpc_inventory (Variables|Default|GetBPC%20Inventory))
  (bind _playerref (Variables|Refs|GetPlayerRef))
  (bind _slotselected (Variables|/Game/Blueprint/BP_Player.BP_Player_C|GetSlotSelected _playerref))
  (bind _element (Default|GetElement _bpc_inventory _slotselected))
  ;[1 1 1] Drop Item
  (:Started
    (if (Variables|/Game/Blueprint/BP_GameMode.BP_GameMode_C|GetHasBackpack (Variables|Refs|GetGameModeRef))
      (if (Utilities|IsValidClass _element)
        (Default|DropItem _bpc_inventory _element)
        (Default|RemoveItemfromInventory _bpc_inventory _slotselected)
        (Audio|PlaySoundatLocation "/Game/Inventory/Sounds/DropItem.DropItem" (Transformation|GetActorLocation (Variables|Refs|GetPlayerRef)) "0, 0, 0" 1.0 1.0 0.0 0 0 0 0)))))

(event EventBeginPlay
  ;[1 1 1] Comment
  (Variables|Refs|SetPlayerCharacterRef (Game|GetPlayerCharacter 0))
  (Variables|Refs|SetPlayerControllerRef (Game|GetPlayerController 0))
  (bind _asbp_game_mode (Utilities|Casting|CastToBP_GameMode (Game|GetGameMode)))
  (bind _output_get (Variables|Refs|SetGameModeRef _asbp_game_mode))
  (Variables|Default|SetBPC%20Inventory (Variables|/Game/Blueprint/BP_GameMode.BP_GameMode_C|GetBPC_inventory _output_get))
  (bind _asbp_player (Utilities|Casting|CastToBP_Player (Variables|Refs|GetPlayerCharacterRef)))
  (Variables|Refs|SetPlayerRef _asbp_player))