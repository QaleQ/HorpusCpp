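; Player character for a stealth horror game, handling movement noise, breathing and interaction detection.
; Timelines drive randomized footstep sounds and AI noise reports for steps and breath, with a clamped sneak level intended to dampen footsteps.
; Tick switches between regular and heavy breathing by monster proximity and line-traces from the camera to show the interact dot and collectable widgets.
; BeginPlay caches game mode references and sets up input and UI.
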(event Custom|Add%20to%20sneakLevel
  (params (SneakLevel :type Float%20%28double-precision%29))
  ;[1 1 1] Set sneakLevel from other classes
  (CallFunction|AddtoSneakLevel SneakLevel))

(event Custom|Set%20Movement%20Input
  (params (NewInput :type Boolean))
  (bind _player_controller_ref (Variables|References|GetPlayer%20Controller%20Ref))
  ;[1 1 1] Called by BP_Hide when interacting with hide objects disables the movement  only.
  (if NewInput
    (Input|SetIgnoreMoveInput _player_controller_ref true)
    (else
      (Input|ResetIgnoreMoveInput _player_controller_ref))))

(event Custom|PlayFootstepTimeline
  (params (NewEnabled :type Boolean))
  (bind _footstepsoundtimeline (Variables|Default|GetFootstepSoundTimeline))
  ;[1 1 1] PlayFootstepTimeline event (called on movement input)
  (if NewEnabled
    (Audio|Components|Audio|Play _footstepsoundtimeline)
    (else
      (Audio|Components|Audio|Stop _footstepsoundtimeline))))

(event EventBeginPlay
  ;[1 1 1] Begin play
  (Utilities|FlowControl|Sequence
    (:then_0
      ;;[1 1 1] Set variables
      (bind _asbp_game_mode (Utilities|Casting|CastToBP_GameMode (Game|GetGameMode)))
      (bind _output_get (Variables|References|SetGameModeRef _asbp_game_mode))
      (Variables|Default|SetBPC%20Inventory (Variables|/Game/Blueprint/BP_GameMode.BP_GameMode_C|GetBPC_inventory _output_get))
      (Variables|References|SetPlayer%20Controller%20Ref (Game|GetPlayerController 0)))
    (:then_1
      ;;[1 1 1] Start breathing sound emission
      (Audio|Components|Audio|Play (Variables|Default|GetEmitBreathSound)))
    (:then_2
      ;;[1 1 1] Set Interact Dot Widget ref
      (bind _returnvalue (UserInterface|CreateWidget "/Game/UI/crosshair/InteractDotWidget.InteractDotWidget_C"))
      (Variables|References|SetInteract%20Dot%20Widget _returnvalue))
    (:then_3
      ;;[1 1 1] Add default mapping context
      (Input|AddMappingContext (PlayerController|LocalPlayerSubsystems|GetEnhancedInputLocalPlayerSubsystem (Variables|References|GetPlayer%20Controller%20Ref)) "/Game/Input/IMC_Default.IMC_Default" 0 "(bIgnoreAllPressedKeysUntilRelease=True,bForceImmediately=False)"))
    (:then_4
      ;;[1 1 1] Get PusRef
      (bind _returnvalue_2 (Actor|GetActorOfClass "/Game/Monsters/BP_Monster_Smart.BP_Monster_Smart_C"))
      (Variables|References|SetMonsterRef _returnvalue_2))
    (:then_5
      ;;[1 1 1] Added AlwaysShownWidget (because all other widgets are used  for specific things
      (bind _returnvalue_3 (UserInterface|CreateWidget "/Game/UI/BPW_AlwaysVisibleUI.BPW_AlwaysVisibleUI_C" (Variables|References|GetPlayer%20Controller%20Ref)))
      (bind _output_get_2 (Variables|References|SetAlwaysVisibleUIRef _returnvalue_3))
      (UserInterface|Viewport|AddtoViewport _output_get_2 0))
    (:then_6
      ;;[1 1 1] Set Inventory slot1 Selected from start
      (Default|OnStartMakeSelectedSlotHighlighted (Variables|Default|GetBPC_PlayerInput)))))

(event EventTick
  (params (DeltaSeconds :type Float%20%28single-precision%29))
  ;[1 1 1] Event Tick
  ;;[1 1 1] Determine breath rate
  (CallFunction|SetBreathRate)
  (bind _hitactor (CallFunction|LineTrace))
  (CallFunction|CheckInteractable _hitactor))

(event Custom|SetBreathRate
  (bind _regularbreathing (Variables|Default|GetRegularBreathing))
  (bind _heavybreathing (Variables|Default|GetHeavyBreathing))
  ;[1 0.08854 0.08854] Change breath rate logic (on tick)
  (bind _monsterref (Variables|References|GetMonsterRef)
    (:then
      (if (< (Transformation|GetDistanceTo _monsterref self) 5e+02)
        (if (Audio|Components|Audio|IsPlaying _regularbreathing)
          (Audio|Components|Audio|Stop _regularbreathing)
          (Audio|Components|Audio|Play (Variables|Default|GetHeavyBreathing) 0.0))
        (elif (Audio|Components|Audio|IsPlaying _heavybreathing)
          (Audio|Components|Audio|Stop _heavybreathing)
          (Audio|Components|Audio|Play (Variables|Default|GetRegularBreathing) 0.0))))
    (:else)))

(fn ConstructionScript)

(fn AddtoSneakLevel
  (params (SneakLevel :type Float%20%28double-precision%29))
  ;[1 1 1] Adds to stealth and is clamped with 1 as max, 0 min
  (bind _output_get (Variables|Default|SetSneakLevel (Math|Float|Clamp(Float) (+ SneakLevel (Variables|Default|GetSneakLevel)))))
  (bind _asbp_game_instance (Utilities|Casting|CastToBP_GameInstance (Game|GetGameInstance)))
  (Default|GetSneakLevel _asbp_game_instance _output_get))

(fn Sneaking
  (params (Condition :type Boolean))
  (bind _footstepsoundtimeline (Variables|Default|GetFootstepSoundTimeline))
  (bind _charactermovement (Variables|Character|GetCharacterMovement))
  (bind _defaultwalkspeed (LocalVariables|GetDefaultWalkSpeed))
  (bind _sneakleveleffect (LocalVariables|GetSneakLevelEffect))
  (bind _defaulttimelineplayrate (LocalVariables|GetDefaultTimelinePlayRate))
  ;[1 1 1] Comment
  (if Condition
    (Variables|/Script/Engine.CharacterMovementComponent|SetMaxWalkSpeed _charactermovement (* _defaultwalkspeed (LocalVariables|GetSneakSpeedModifier)))
    (CallFunction|AddtoSneakLevel _sneakleveleffect)
    (Components|Timeline|SetPlayRate _footstepsoundtimeline (* _defaulttimelineplayrate (LocalVariables|GetSneakSpeedModifier)))
    (else
      (Variables|/Script/Engine.CharacterMovementComponent|SetMaxWalkSpeed _charactermovement _defaultwalkspeed)
      (CallFunction|AddtoSneakLevel (* _sneakleveleffect -1.0))
      (Components|Timeline|SetPlayRate _footstepsoundtimeline _defaulttimelineplayrate))))

(fn LineTrace
  (bind _camera (Variables|Default|GetCamera))
  (bind _returnvalue (Transformation|GetWorldLocation _camera))
  (bind _outhit (Collision|LineTraceByChannel _returnvalue (+ _returnvalue (* (Math|Vector|GetForwardVector _camera) (Variables|DefaultValues|GetInteractDistance))) "TraceTypeQuery1" false 0 "None"))
  (return (.HitActor (Collision|BreakHitResult _outhit))))

(fn CheckInteractable
  (params (HitActor :type Object%20Object%20Reference))
  (bind _interact_dot_widget (Variables|References|GetInteract%20Dot%20Widget))
  ;[1 1 1] If hit actor implements Interactable
  (if (Utilities|DoesObjectImplementInterface HitActor "/Game/Interactable/BPI_Interactable.BPI_Interactable_C")
    ;[1 1 1] If dot is not in viewport
    (if (not (UserInterface|Viewport|IsinViewport (Variables|References|GetInteract%20Dot%20Widget)))
      ;[1 1 1] Draw dot
      (UserInterface|Viewport|AddtoViewport _interact_dot_widget 0)
      ;[1 1 1] Toggle item widget
      (bind _asbp_collectable (Utilities|Casting|CastToBP_Collectable HitActor))
      (bind _output_get (Variables|Default|SetHitActorWidget (Variables|/Game/Interactable/Collectable/BP_Collectable.BP_Collectable_C|GetWidget _asbp_collectable)))
      (Development|SetHiddeninGame _output_get false false))
    (else
      ;[1 1 1] Remove dot
      (Widget|RemovefromParent _interact_dot_widget)
      (Variables|Default|GetHitActorWidget
        (:then
          (Development|SetHiddeninGame _output_get true false))
        (:else)))))