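; BP_Hide is an interactable hiding place that moves the player in and out of a hidden spot.
; Interact, allowed while the player overlaps or is hidden, flip-flops a timeline forward and in reverse.
; Separate lateral and vertical alphas interpolate the player between their saved position and the HidingPlaceBox.
; A direction-checked timeline event toggles movement input, collision and capsule height, and stops footstep sounds when hiding.
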(event Custom|SetPlayerMovement
  (params (NewMovement :type Boolean))
  (bind _playerref (Variables|Default|GetPlayerRef))
  (bind _capsulecomponent (Variables|/Script/Engine.Character|GetCapsuleComponent _playerref))
  ;[1 1 1] Hide
  ;;[1 1 1] Enable/Disable movement, collision and step sounds, change height
  (if NewMovement
    (Default|SetMovementInput _playerref false)
    (Collision|SetActorEnableCollision _playerref true)
    (Variables|Default|SetOutsideOfHidingplace true)
    ;;;[1 0 0] To prevent going below navmesh
    (Components|Capsule|SetCapsuleHalfHeight _capsulecomponent 88.0 true)
    (else
      (Default|SetMovementInput _playerref true)
      (Audio|Components|Audio|Stop (Variables|/Game/Blueprint/BP_Player.BP_Player_C|GetFootstepSoundTimeline _playerref))
      (Collision|SetActorEnableCollision _playerref false)
      (Variables|Default|SetOutsideOfHidingplace false)
      (Components|Capsule|SetCapsuleHalfHeight _capsulecomponent 39.0 false))))

(event EventInteract
  (bind _hidingplacelocation (Variables|Default|GetHidingPlaceLocation))
  ;[1 1 1] Hide
  (if (or (Variables|Default|GetInteractEnabled) (not (Variables|Default|GetOutsideOfHidingplace)))
    (Utilities|FlowControl|FlipFlop
      (:A
        (bind (_direction _lateralalpha _verticalalpha) (Timeline|Timeline Play)
          (:Update
            ;;[1 1 1] Move player
            (Transformation|SetActorLocation (Variables|Default|GetPlayerRef) (Math|Vector|MakeVector (.x (Math|Vector|Lerp(Vector) (Math|Vector|MakeVector (.x (Variables|Default|GetOriginalPlayerLocation)) (.y (Variables|Default|GetOriginalPlayerLocation)) 0.0) (Math|Vector|MakeVector (.x _hidingplacelocation) (.y _hidingplacelocation) 0.0) _lateralalpha)) (.y (Math|Vector|Lerp(Vector) (Math|Vector|MakeVector (.x (Variables|Default|GetOriginalPlayerLocation)) (.y (Variables|Default|GetOriginalPlayerLocation)) 0.0) (Math|Vector|MakeVector (.x _hidingplacelocation) (.y _hidingplacelocation) 0.0) _lateralalpha)) (Math|Float|Lerp (.z (Variables|Default|GetOriginalPlayerLocation)) (.z _hidingplacelocation) _verticalalpha)) false false))
          (:AnimationStartPoint
            (switch Utilities|FlowControl|Switch|SwitchonETimelineDirection _direction
              (:Forward
                ;;[1 1 1] Hiding start
                (Variables|Default|SetOriginalPlayerLocation (Transformation|GetActorLocation (Variables|Default|GetPlayerRef)))
                (CallFunction|SetPlayerMovement false))
              (:Backward
                ;;[1 1 1] Hiding stop
                (CallFunction|SetPlayerMovement true))))))
      (:B
        (Timeline|Timeline Reverse)))))

(event Collision|EventActorBeginOverlap
  (params (OtherActor :type Actor%20Object%20Reference))
  ;[1 1 1] Enable/disable interact based on player begin/end overlap
  (if (== OtherActor (Game|GetPlayerCharacter 0))
    (Variables|Default|SetInteractEnabled true)))

(event Collision|EventActorEndOverlap
  (params (OtherActor :type Actor%20Object%20Reference))
  ;[1 1 1] Enable/disable interact based on player begin/end overlap
  (if (== (Game|GetPlayerCharacter 0) OtherActor)
    (Variables|Default|SetInteractEnabled false)))

(event EventBeginPlay
  ;[1 1 1] Set variables on BeginPlay
  (Variables|Default|SetHidingPlaceLocation (Transformation|GetWorldLocation (Variables|Default|GetHidingPlaceBox)))
  (bind _asbp_player (Utilities|Casting|CastToBP_Player (Game|GetPlayerCharacter 0)))
  (Variables|Default|SetPlayerRef _asbp_player))

(fn ConstructionScript)